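; BP_EntryController sets up the game's entry screen.
; On BeginPlay it creates the WBP_Entry widget for the first player controller, adds it to the viewport and shows the mouse cursor.
; A debug key prints the current and maximum resolution scale from GameUserSettings.
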(event EventBeginPlay
  (bind _returnvalue (UserInterface|CreateWidget "/Game/Entry/WBP_Entry.WBP_Entry_C" (Game|GetPlayerController 0)))
  (UserInterface|Viewport|AddtoViewport _returnvalue 0)
  (Variables|/Script/Engine.PlayerController|SetbShowMouseCursor (Game|GetPlayerController 0) true))

(event EventTick
  (params (DeltaSeconds :type Float%20%28single-precision%29)))

(event Input|KeyboardEvents|DebugKey1
  (params (Key :type Key%20Structure :default "None") (ActionValue :type Input%20Action%20Value%20Structure))
  (:Pressed
    (bind _returnvalue (Settings|GetGameUserSettings))
    (Development|PrintString (Utilities|String|Append "Render Res: " (Utilities|String|ToString(Float) (.CurrentScaleValue (Class|GameUserSettings|GetResolutionScaleInformationEx _returnvalue))) " Max: " (Utilities|String|ToString(Float) (.MaxScaleValue (Class|GameUserSettings|GetResolutionScaleInformationEx _returnvalue)))))))

(fn ConstructionScript)