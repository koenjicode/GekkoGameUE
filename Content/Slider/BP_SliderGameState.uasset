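; Game state for a slider game that displays four colored cubes through a fixed orthographic camera.
; BeginPlay spawns the cubes, each with a dynamic material tinted by index, then spawns the camera and makes it the view target next tick.
; While unpaused, Tick sets each cube's horizontal position from scaled game positions and stacks them vertically by cube size.
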(event `self.ReceiveBeginPlay`
  (`parent.ReceiveBeginPlay`)
  (`self.CreateCubes`)
  (bind _returnvalue (`|SpawnActorFromClass` "/Script/Engine.CameraActor" (`KismetMathLibrary.MakeTransform` (0.0 123.0 -60.0)) "Undefined" "MultiplyWithRoot" null null))
  (set `self.Camera` _returnvalue)
  (`CameraComponent.SetProjectionMode` (`CameraActor.CameraComponent` (`self.Camera`)) "Orthographic")
  (`CameraComponent.SetOrthoWidth` (`CameraActor.CameraComponent` (`self.Camera`)) 285.0)
  (`KismetSystemLibrary.DelayUntilNextTick`)
  (`PlayerController.SetViewTargetWithBlend` (`GameplayStatics.GetPlayerController` 0) (`self.Camera`) 0.0 "VTBlend_Linear" 0.0 false))

(event `self.ReceiveTick`
  (params (DeltaSeconds :type "Float (single-precision)"))
  (`parent.ReceiveTick` DeltaSeconds)
  (if (not (`self.bPaused`))
    (if (== (`KismetArrayLibrary.Array_Length` (`self.Cubes`)) 4)
      (`self.UpdateView`))))

(fn `CreateCubes`
  (locals (NewCube :type "/Game/Slider/BP_SliderCube Object Reference") (NewLocalVar :type "MaterialInstanceDynamic Object Reference") (InCubeIndex :type Integer))
  (for _index (range 4)
    (set `local.InCubeIndex` _index)
    (bind _returnvalue (`|SpawnActorFromClass` "/Game/Slider/BP_SliderCube.BP_SliderCube_C" (`self.GetTransform`) "Undefined" "MultiplyWithRoot" null null))
    (bind _output_get (set `local.NewCube` _returnvalue))
    (bind _returnvalue_2 (`PrimitiveComponent.CreateDynamicMaterialInstance` (`/Game/Slider/BP_SliderCube.Cube` _output_get) 0 "/Game/Slider/MI_CubeMat.MI_CubeMat" "None"))
    (`MaterialInstanceDynamic.SetVectorParameterValue` _returnvalue_2 "Color" (`self.GetMaterialColor` (`local.InCubeIndex`)))
    (`KismetArrayLibrary.Array_Add` (`self.Cubes`) (`local.NewCube`))))

(fn `UpdateView`
  (locals (InCube :type "/Game/Slider/BP_SliderCube Object Reference") (InUpdateIndex :type Integer))
  (for _index (range (`KismetArrayLibrary.Array_Length` (`self.Cubes`)))
    (set `local.InUpdateIndex` _index)
    (bind _output_get (set `local.InCube` (`|GetArrayItem` (`self.Cubes`) (`local.InUpdateIndex`))))
    (`self.K2_SetActorLocation` _output_get (`KismetMathLibrary.MakeVector` 0.0 (/ (.x (/ (`self.GetCubePosition` (`local.InUpdateIndex`)) (`self.GetSliderGameScale`))) (`self.UnrealScale`)) (* (* (* (.x (`SceneComponent.K2_GetComponentScale` (`/Game/Slider/BP_SliderCube.Cube` (`local.InCube`)))) 100.0) (`local.InUpdateIndex`)) -1.0)) false false)))

(fn `UserConstructionScript`)