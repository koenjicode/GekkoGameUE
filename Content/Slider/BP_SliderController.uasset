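; BP_SliderController is a player controller for the Slider game that records session state and offers a debug exit from a GekkoNet session.
; On BeginPlay it caches the GekkoGameState, whether a GekkoNet session is running, and whether it is player controller index 0.
; A debug key on that first controller ends the session and opens the L_Entry level.
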(event EventBeginPlay
  (Variables|Default|SetGekkoGameState (.AsGekko%20Game%20State (Utilities|Casting|CastToGekkoGameState (Game|GetGameState))))
  (Variables|Default|SetbIsOnline (Class|GekkoNetSubsystem|IsSessionRunning (Subsystems|GetGekkoNetSubsystem)))
  (bind _output_get (Variables|Default|SetbFirstController (== (Game|GetPlayerController 0) self)))
  (if _output_get
    _))

(event Input|KeyboardEvents|DebugKey4
  (params (Key :type Key%20Structure :default "None") (ActionValue :type Input%20Action%20Value%20Structure))
  (:Pressed
    (if (Variables|Default|GetbFirstController)
      (Class|GekkoNetSubsystem|EndSession (Subsystems|GetGekkoNetSubsystem))
      (Game|OpenLevel(byObjectReference) "/Game/OnlineSession/L_Entry.L_Entry"))))

(fn ConstructionScript)