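; BP_ServerGameState is a network-test game state that passes a client's local delay amount toward the server.
; On BeginPlay without authority, it calls Client_SendCharacterInfo, which reads LocalDelayAmount from BP_GekkoGameInstance.
; That value goes to Recieve_SendCharacterInfo, which only prints it with a message saying the server will have the info.
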(event `self.ReceiveBeginPlay`
  (`/Engine/EditorBlueprintResources/ActorMacros.Switch Has Authority`
    (:`Remote`
      (`self.Client_SendCharacterInfo`))))

(event `Client_SendCharacterInfo`
  (`self.Recieve_SendCharacterInfo` (`GekkoGameInstance.LocalDelayAmount` (cast `/Game/OnlineSession/BP_GekkoGameInstance` (`GameplayStatics.GetGameInstance`) :!pure true))))

(event `Recieve_SendCharacterInfo`
  (params (Delay :type Integer))
  (`KismetSystemLibrary.PrintString` (`KismetStringLibrary.Concat_StrStr` "The Server will have your info: " (`KismetStringLibrary.Conv_IntToString` Delay))))

(fn `UserConstructionScript`)