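; BP_ServerTestController is a network test controller that relays a hello between players through the server.
; DebugKey1 triggers SendHello, which passes a string and the local PlayerId to a server handler.
; The server loops over PlayerArray and calls the client handler on every other player's controller.
; That handler receives the recipient's own PlayerId, so the printed message names the receiver; the string is unused.
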(event Custom|SendHello
  (Development|PrintString "Sending Hello")
  (CallFunction|ServerHandleHello "Hello!" (Variables|/Script/Engine.PlayerState|GetPlayerId (Variables|GetPlayerState))))

(event Custom|Server_HandleHello
  (params (InString :type String) (Sender :type Integer))
  (for _array_element (Variables|/Script/Engine.GameStateBase|GetPlayerArray (Game|GetGameState))
    (if (!= (Variables|/Script/Engine.PlayerState|GetPlayerId _array_element) Sender)
      (CallFunction|ClientHandleHello (.AsBP%20Server%20Test%20Controller (Utilities|Casting|CastToBP_ServerTestController (Game|GetPlayerController _array_element))) (Variables|/Script/Engine.PlayerState|GetPlayerId _array_element)))))

(event Custom|Client_HandleHello
  (params (Sender :type Integer))
  (Development|PrintString (Utilities|String|Append "Recieved a hello from Client " (Utilities|String|ToString(Integer) Sender))))

(event EventBeginPlay)

(event EventTick
  (params (DeltaSeconds :type Float%20%28single-precision%29)))

(event Input|KeyboardEvents|DebugKey1
  (params (Key :type Key%20Structure :default "None") (ActionValue :type Input%20Action%20Value%20Structure))
  (:Pressed
    (CallFunction|SendHello)))

(fn ConstructionScript)