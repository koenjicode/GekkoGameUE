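; Game instance that manages the online session lifecycle: creating, finding and joining, and leaving sessions, with LAN and lobby options.
; Creating a session opens the chosen level as a listen server, while searching automatically joins the first result without any selection.
; Leaving destroys the session and returns to L_Entry.
; Network and travel errors print the failure type and share a path that destroys the session without loading a level.
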(event `CreateSession`
  (params (PlayerController :type "PlayerController Object Reference") (PublicConnections :type Integer) (bUseLAN :type Boolean) (bUseLobbiesIfAvailable :type Boolean) (LevelToTravelTo :type "World Soft Object Reference"))
  ; Create and Joining
  (`CreateSessionCallbackProxy.CreateSession` PlayerController PublicConnections bUseLAN bUseLobbiesIfAvailable
    (:`OnSuccess`
      (`GameplayStatics.OpenLevelBySoftObjectPtr` LevelToTravelTo true "listen"))))

(event `FindSession`
  (params (PlayerController :type "PlayerController Object Reference") (MaxResults :type Integer) (bUseLAN :type Boolean) (bUseLobbies :type Boolean))
  ; Create and Joining
  (bind _results (`FindSessionsCallbackProxy.FindSessions` PlayerController MaxResults bUseLAN bUseLobbies)
    (:`OnSuccess`
      (`JoinSessionCallbackProxy.JoinSession` (`GameplayStatics.GetPlayerController` 0) (`|GetArrayItem` _results)))))

(event `LeaveSession`
  (params (PlayerController :type "PlayerController Object Reference"))
  ; Destroying Session
  (`DestroySessionCallbackProxy.DestroySession` PlayerController
    (:`OnSuccess`
      (`GameplayStatics.OpenLevelBySoftObjectPtr` "/Game/OnlineSession/L_Entry.L_Entry"))))

(event `self.HandleNetworkError`
  (params (FailureType :type "ENetworkFailure Enum" :default "NetDriverAlreadyExists") (bIsServer :type Boolean))
  ; Destroying Session
  (`KismetSystemLibrary.PrintString` (`|GetEnumeratorNameAsString` FailureType))
  (`DestroySessionCallbackProxy.DestroySession` (`GameplayStatics.GetPlayerController` 0) :!label _label))

(event `self.HandleTravelError`
  (params (FailureType :type "ETravelFailure Enum" :default "NoLevel"))
  ; Destroying Session
  (`KismetSystemLibrary.PrintString` (`|GetEnumeratorNameAsString` FailureType))
  (goto _label))