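; BP_GekkoBaseController is a player controller for GekkoNet sessions that handles pausing and online debug hotkeys.
; On BeginPlay it flags whether it is the first local controller, which alone can toggle GekkoBaseState pause, and only while offline.
; Debug keys adjust local input delay through the GekkoNet subsystem with runahead adjustment, simulate a player disconnect, and print player ID and opponent address.
; IsOnline counts either a running GekkoNet session or non-standalone mode as online.
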(event EventBeginPlay
  (bind _output_get (Variables|Default|SetbFirstController (== (Game|GetPlayerController 0) self)))
  (if _output_get
    _))

(event Input|KeyboardEvents|DebugKey4
  (params (Key :type Key%20Structure :default "None") (ActionValue :type Input%20Action%20Value%20Structure))
  ;[0.15 0.15 0.15 0.5] Debug: Online Shutdown
  (:Pressed
    (if (Variables|Default|GetbFirstController)
      (Class|GekkoGameState|PlayerDisconnected (.AsGekko%20Base%20State (Utilities|Casting|CastToGekkoBaseState (Game|GetGameState)))))))

(event Input|KeyboardEvents|DebugKey7
  (params (Key :type Key%20Structure :default "None") (ActionValue :type Input%20Action%20Value%20Structure))
  (:Pressed
    (Development|PrintString (Utilities|String|Append "Opponent: " (Class|GekkoPlayerController|GetOpponentAddressasString)))))

(event Input|KeyboardEvents|DebugKey1
  (params (Key :type Key%20Structure :default "None") (ActionValue :type Input%20Action%20Value%20Structure))
  ;[0.15 0.15 0.15 0.5] Debug: Online Delay
  (:Pressed
    (CallFunction|SetLocalDelay (+ (CallFunction|GetCurrentDelay) 1))))

(event Input|KeyboardEvents|DebugKey2
  (params (Key :type Key%20Structure :default "None") (ActionValue :type Input%20Action%20Value%20Structure))
  ;[0.15 0.15 0.15 0.5] Debug: Online Delay
  (:Pressed
    (CallFunction|SetLocalDelay (- (CallFunction|GetCurrentDelay) 1))))

(event Input|KeyboardEvents|DebugKey6
  (params (Key :type Key%20Structure :default "None") (ActionValue :type Input%20Action%20Value%20Structure))
  (:Pressed
    (Development|PrintString (Utilities|String|Append "ID: " (Class|AdvancedSessionsLibrary|UniqueNetIdtoString (Class|AdvancedSessionsLibrary|GetUniqueNetIDfromPlayerState (Variables|/Script/Engine.Controller|GetPlayerState (Game|GetPlayerController 0))))))
    (Development|PrintString (Utilities|GetDisplayName (Game|GetPlayerController 0)))))

(event Input|KeyboardEvents|SpaceBar
  (params (Key :type Key%20Structure :default "None"))
  ;[0.15 0.15 0.15 0.5] Pause
  (:Pressed
    (if (and (Variables|Default|GetbFirstController) (not (CallFunction|IsOnline)))
      (Class|GekkoGameState|TogglePause (.AsGekko%20Base%20State (Utilities|Casting|CastToGekkoBaseState (Game|GetGameState)))))))

(fn ConstructionScript)

(fn SetLocalDelay
  (params (Delay :type Integer))
  (Class|GekkoNetSubsystem|SetLocalDelay (Subsystems|GetGekkoNetSubsystem) Delay (Variables|/Script/GekkoGameUE.GekkoGameState|GetNetLocalPlayerID (Variables|Default|GetGekkoGameState)) true))

(fn GetCurrentDelay
  (return (.Delay (Utilities|Struct|BreakGekkoNetworkStats (Variables|/Script/GekkoGameUE.GekkoGameState|GetNetStats (Variables|Default|GetGekkoGameState))))))

(fn IsOnline
  (return (or (Class|GekkoNetSubsystem|IsSessionRunning (Subsystems|GetGekkoNetSubsystem)) (not (Class|KismetSystemLibrary|IsStandalone)))))