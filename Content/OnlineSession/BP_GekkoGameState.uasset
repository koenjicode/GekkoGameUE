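; Game state for an online Pong game that acts as the visual layer for simulated ball and paddle positions.
; On BeginPlay, Init spawns the ball, two paddles and an orthographic camera, which non-dedicated instances set as their view.
; OnUnrealDraw copies simulation positions onto those actors, printing a warning for NaN vectors.
; PlayerDisconnected leaves the session or, in standalone, opens the entry level, while Tick logs player count changes.
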(event `self.ReceiveBeginPlay`
  (`self.Init`)
  (`parent.ReceiveBeginPlay`))

(event `self.OnUnrealDraw`
  (bind _returnvalue (`self.GetBallPosition` 0))
  (if (`KismetMathLibrary.Vector_IsNAN` _returnvalue)
    (`KismetSystemLibrary.PrintString` "Bad Ball Pos!!!" true true (struct :`R` 1.0 :`G` 0.013929 :`B` 0.032916 :`A` 1.0))
    (else
      (`self.K2_SetActorLocation` (`self.Ball`) _returnvalue false false)
      (for _index (range 2)
        (bind _returnvalue_2 (`self.GetPaddlePosition` _index))
        (if (`KismetMathLibrary.Vector_IsNAN` _returnvalue_2)
          (`KismetSystemLibrary.PrintString` (`KismetStringLibrary.Concat_StrStr` "Bad Paddle Vector!!! " (`KismetStringLibrary.Conv_IntToString` _index)) true true (struct :`R` 1.0 :`G` 0.006285 :`A` 1.0))
          (else
            (`self.K2_SetActorLocation` (`|GetArrayItem` (`self.Paddles`) _index) _returnvalue_2 false false)))))))

(event `self.PlayerDisconnected`
  (params (Handle :type Integer))
  ; Close Session on Disconnect
  (if (not (`KismetSystemLibrary.IsStandalone`))
    (`/Game/OnlineSession/BP_GekkoGameInstance.LeaveSession` (cast `/Game/OnlineSession/BP_GekkoGameInstance` (`GameplayStatics.GetGameInstance`) :!pure true))
    (else
      (`GameplayStatics.OpenLevelBySoftObjectPtr` "/Game/OnlineSession/L_Entry.L_Entry"))))

(event `self.ReceiveTick`
  (params (DeltaSeconds :type "Float (single-precision)"))
  (`parent.ReceiveTick` DeltaSeconds)
  (`|ExecutionSequence`
    (:`then_0`
      (if (!= (`KismetArrayLibrary.Array_Length` (`self.PlayerArray`)) (`self.LastPlayerArrayCount`))
        (`KismetSystemLibrary.PrintString` (`KismetStringLibrary.Concat_StrStr` "New Player Array Size: " (`KismetStringLibrary.Conv_IntToString` (`KismetArrayLibrary.Array_Length` (`self.PlayerArray`)))) true true (struct :`G` 0.66 :`B` 1.0 :`A` 1.0) 4.0)))
    (:`then_1`
      (set `self.LastPlayerArrayCount` (`KismetArrayLibrary.Array_Length` (`self.PlayerArray`))))))

(fn `Init`
  (locals (SpawnedPaddle :type "/Game/OnlineSession/Draw/BP_PongPaddle Object Reference"))
  (`|ExecutionSequence`
    (:`then_0`
      ; Ball
      (bind _returnvalue (`|SpawnActorFromClass` "/Game/OnlineSession/Draw/BP_PongBall.BP_PongBall_C" (`self.GetTransform`) "Undefined" "MultiplyWithRoot" null null))
      (set `self.Ball` _returnvalue)
      ; Paddles
      (for _ (range 2)
        (bind _returnvalue_2 (`|SpawnActorFromClass` "/Game/OnlineSession/Draw/BP_PongPaddle.BP_PongPaddle_C" (`self.GetTransform`) "Undefined" "MultiplyWithRoot" null null))
        (set `local.SpawnedPaddle` _returnvalue_2)
        (`KismetArrayLibrary.Array_Add` (`self.Paddles`) (`local.SpawnedPaddle`))))
    (:`then_1`
      ; Camera
      (bind _returnvalue_3 (`|SpawnActorFromClass` "/Script/Engine.CameraActor" (`KismetMathLibrary.MakeTransform` (300.0 0.0 300.0) (struct :`Yaw` 90.0 :`Roll` 180.0)) "Undefined" "MultiplyWithRoot" null null))
      (set `self.Camera` _returnvalue_3)
      (`CameraComponent.SetProjectionMode` (`CameraActor.CameraComponent` (`self.Camera`)) "Orthographic")
      (`CameraComponent.SetOrthoWidth` (`CameraActor.CameraComponent` (`self.Camera`)) 1075.0)
      (if (not (`KismetSystemLibrary.IsDedicatedServer`))
        (`PlayerController.SetViewTargetWithBlend` (`GameplayStatics.GetPlayerController` 0) (`self.Camera`) 0.0 "VTBlend_Linear" 0.0 false)))))

(fn `UserConstructionScript`)