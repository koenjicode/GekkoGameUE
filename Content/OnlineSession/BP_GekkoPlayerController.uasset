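; Player controller for Gekko rollback-netcode matches that creates the game HUD and handles offline pause plus debug hotkeys.
; Replay keys step or hold-to-scrub frames through GekkoGameState, using a retriggerable delay to detect holds that Tick continues, and toggle or rewind replay takeover.
; Online keys adjust local input delay, toggle detailed network stats, or end the session and return to the entry level.
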(event EventBeginPlay
  ;[0.15 0.15 0.15 0.5] Begin Play
  (Variables|Default|SetGekkoGameState (.AsGekko%20Game%20State (Utilities|Casting|CastToGekkoGameState (Game|GetGameState))))
  (Variables|Default|SetReplayManager (Class|GekkoGameState|GetReplayManager (.AsGekko%20Game%20State (Utilities|Casting|CastToGekkoGameState (Game|GetGameState)))))
  (Utilities|FlowControl|DelayUntilNextTick)
  (Utilities|FlowControl|Sequence
    (:then_0
      (Utilities|IsValid (Variables|Default|GetReplayManager)
        (:Is%20Valid
          (Variables|Default|SetbControllingReplay (Class|RedoReplayManager|IsPlayingBackReplay (Variables|Default|GetReplayManager))))))
    (:then_1
      (Variables|Default|SetbIsOnline (Class|GekkoNetSubsystem|IsSessionRunning (Subsystems|GetGekkoNetSubsystem)))
      (bind _output_get (Variables|Default|SetbFirstController (== (Game|GetPlayerController 0) self)))
      (if _output_get
        (bind _returnvalue (UserInterface|CreateWidget "/Game/OnlineSession/WBP_GekkoGame_HUD.WBP_GekkoGame_HUD_C" (Game|GetPlayerController 0)))
        (bind _output_get_2 (Variables|Default|SetHud _returnvalue))
        (UserInterface|Viewport|AddtoViewport _output_get_2 0)
        (Variables|/Game/OnlineSession/WBP_GekkoGame_NetworkStatsDetailed.WBP_GekkoGame_NetworkStatsDetailed_C|SetTargetID (Variables|/Game/OnlineSession/WBP_GekkoGame_HUD.WBP_GekkoGame_HUD_C|GetDetailedNetworkStats (Variables|Default|GetHud)) (Math|Integer|SelectInt 1 0 (== (Variables|/Script/GekkoGameUE.GekkoGameInstance|GetPlayerId (.AsGekko%20Game%20Instance (Utilities|Casting|CastToGekkoGameInstance (Game|GetGameInstance)))) 0)))))))

(event EventTick
  (params (DeltaSeconds :type Float%20%28single-precision%29))
  (bind _returnvalue (Game|GetPlayerController 0))
  (bind _returnvalue_2 (Game|GetPlayerController 0))
  (bind _gekkogamestate (Variables|Default|GetGekkoGameState))
  (bind _returnvalue_3 (Game|Player|IsInputKeyDown _returnvalue "RightShift"))
  (bind _returnvalue_4 (Game|Player|IsInputKeyDown _returnvalue_2 "LeftShift"))
  (bind _returnvalue_5 (or _returnvalue_4 _returnvalue_3))
  (bind _returnvalue_6 (Math|Integer|SelectInt 2 1 _returnvalue_5))
  ;[0.15 0.15 0.15 0.5] Tick
  (if (Variables|Default|GetbControllingReplay)
    (if (Variables|Default|GetbRewindHeld)
      (if (Game|Player|IsInputKeyDown (Game|GetPlayerController 0) "Eight")
        (Class|GekkoGameState|RewindBackfromCurrentFrame _gekkogamestate _returnvalue_6)
        (else
          (Class|GekkoGameState|FastForwardfromCurrentFrame _gekkogamestate _returnvalue_6))))))

(event Input|KeyboardEvents|DebugKey4
  (params (Key :type Key%20Structure :default "None") (ActionValue :type Input%20Action%20Value%20Structure))
  ;[0.15 0.15 0.15 0.5] Debug: Online Shutdown
  (:Pressed
    (if (Variables|Default|GetbFirstController)
      (Class|GekkoNetSubsystem|EndSession (Subsystems|GetGekkoNetSubsystem))
      (Game|OpenLevel(byObjectReference) "/Game/OnlineSession/L_Entry.L_Entry"))))

(event Input|KeyboardEvents|DebugKey3
  (params (Key :type Key%20Structure :default "None") (ActionValue :type Input%20Action%20Value%20Structure))
  ;[0.15 0.15 0.15 0.5] Debug: Online Network Stats
  (:Pressed
    (if (Variables|Default|GetbFirstController)
      (if (Variables|Default|GetbIsOnline)
        (Widget|SetVisibility (Variables|/Game/OnlineSession/WBP_GekkoGame_HUD.WBP_GekkoGame_HUD_C|GetDetailedNetworkStats (Variables|Default|GetHud)) (select (Widget|IsVisible (Variables|/Game/OnlineSession/WBP_GekkoGame_HUD.WBP_GekkoGame_HUD_C|GetDetailedNetworkStats (Variables|Default|GetHud))) "Hidden" "Visible"))))))

(event Input|KeyboardEvents|DebugKey1
  (params (Key :type Key%20Structure :default "None") (ActionValue :type Input%20Action%20Value%20Structure))
  ;[0.15 0.15 0.15 0.5] Debug: Online Delay
  (:Pressed
    (CallFunction|SetLocalDelay (+ (CallFunction|GetCurrentDelay) 1))))

(event Input|KeyboardEvents|DebugKey2
  (params (Key :type Key%20Structure :default "None") (ActionValue :type Input%20Action%20Value%20Structure))
  ;[0.15 0.15 0.15 0.5] Debug: Online Delay
  (:Pressed
    (CallFunction|SetLocalDelay (- (CallFunction|GetCurrentDelay) 1))))

(event Input|KeyboardEvents|DebugKey9
  (params (Key :type Key%20Structure :default "None") (ActionValue :type Input%20Action%20Value%20Structure))
  ;[0.15 0.15 0.15 0.5] Debug: Replay Controls
  (:Pressed
    (Variables|Default|SetbRewindPressed true)
    (if (Variables|Default|GetbControllingReplay)
      (if (Variables|Default|GetbFirstController)
        (Class|GekkoGameState|FastForwardfromCurrentFrame (.AsGekko%20Game%20State (Utilities|Casting|CastToGekkoGameState (Game|GetGameState))) (Math|Integer|SelectInt (Math|Integer|SelectInt 60 1 (Game|Player|IsInputKeyDown (Game|GetPlayerController 0) "LeftShift")) 60 (Variables|/Script/GekkoGameUE.GekkoGameState|GetbGamePaused (Variables|Default|GetGekkoGameState))))
        (Utilities|FlowControl|RetriggerableDelay 0.4)
        (if (Variables|Default|GetbRewindPressed)
          (Variables|Default|SetbRewindHeld true)))))
  (:Released
    (Variables|Default|SetbRewindPressed false)
    (Variables|Default|SetbRewindHeld false)))

(event Input|KeyboardEvents|DebugKey8
  (params (Key :type Key%20Structure :default "None") (ActionValue :type Input%20Action%20Value%20Structure))
  ;[0.15 0.15 0.15 0.5] Debug: Replay Controls
  (:Pressed
    (Variables|Default|SetbRewindPressed true)
    (if (Variables|Default|GetbControllingReplay)
      (if (Variables|Default|GetbFirstController)
        (Class|GekkoGameState|RewindBackfromCurrentFrame (.AsGekko%20Game%20State (Utilities|Casting|CastToGekkoGameState (Game|GetGameState))) (Math|Integer|SelectInt (Math|Integer|SelectInt 60 1 (Game|Player|IsInputKeyDown (Game|GetPlayerController 0) "LeftShift")) 60 (Variables|/Script/GekkoGameUE.GekkoGameState|GetbGamePaused (Variables|Default|GetGekkoGameState))))
        (Utilities|FlowControl|RetriggerableDelay 0.4)
        (if (Variables|Default|GetbRewindPressed)
          (Variables|Default|SetbRewindHeld true)))))
  (:Released
    (Variables|Default|SetbRewindPressed false)
    (Variables|Default|SetbRewindHeld false)))

(event Input|KeyboardEvents|DebugKey0
  (params (Key :type Key%20Structure :default "None") (ActionValue :type Input%20Action%20Value%20Structure))
  (bind _returnvalue (Game|GetGameState))
  (bind _asgekko_game_state (Utilities|Casting|CastToGekkoGameState _returnvalue))
  ;[0.15 0.15 0.15 0.5] Debug: Replay Takeover
  (:Pressed
    (if (Variables|/Script/GekkoGameUE.GekkoGameState|GetbReplayTakeoverEnabled _asgekko_game_state)
      (Class|GekkoGameState|EndTakeover _asgekko_game_state)
      (else
        (Class|GekkoGameState|TakeoverReplay (.AsGekko%20Game%20State (Utilities|Casting|CastToGekkoGameState (Game|GetGameState))))))))

(event Input|KeyboardEvents|DebugKeyEquals
  (params (Key :type Key%20Structure :default "None") (ActionValue :type Input%20Action%20Value%20Structure))
  ;[0.15 0.15 0.15 0.5] Debug: Replay Takeover
  (:Pressed
    (Class|GekkoGameState|RewindtoTakeoverSnapshot (.AsGekko%20Game%20State (Utilities|Casting|CastToGekkoGameState (Game|GetGameState))))))

(event Input|KeyboardEvents|SpaceBar
  (params (Key :type Key%20Structure :default "None"))
  ;[0.15 0.15 0.15 0.5] Pause
  (:Pressed
    (if (and (Variables|Default|GetbFirstController) (not (Variables|Default|GetbIsOnline)))
      (Class|GekkoGameState|TogglePause (.AsGekko%20Game%20State (Utilities|Casting|CastToGekkoGameState (Game|GetGameState)))))))

(fn ConstructionScript)

(fn SetLocalDelay
  (params (Delay :type Integer))
  (Class|GekkoNetSubsystem|SetLocalDelay (Subsystems|GetGekkoNetSubsystem) Delay (Variables|/Script/GekkoGameUE.GekkoGameState|GetNetLocalPlayerID (Variables|Default|GetGekkoGameState))))

(fn GetCurrentDelay
  (return (.Delay (Utilities|Struct|BreakGekkoSimpleNetworkStats (Variables|/Script/GekkoGameUE.GekkoGameState|GetNetStats (Variables|Default|GetGekkoGameState))))))