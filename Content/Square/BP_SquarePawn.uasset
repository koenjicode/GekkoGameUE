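; BP_SquarePawn is a cube pawn that adds to a coin count on input A and shows it on a player tag.
; OnFixedTick increments Counter while A is held, limited by a countdown timer in ticks.
; OnViewTick handles display separately from that logic, showing the tag only when the count is above zero.
; SetDefaultColor tints the cube through a dynamic material instance.
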(event `self.ReceiveBeginPlay`
  (`SceneComponent.SetVisibility` (`self.PlayerTag`) false false))

(event `self.SetDefaultColor`
  (params (Color :type "LinearColor Structure"))
  (set `self.CubeColor` Color)
  (bind _returnvalue (`PrimitiveComponent.CreateDynamicMaterialInstance` (`self.Cube`) 0 "/Game/Slider/M_CubeMat.M_CubeMat" "None"))
  (`MaterialInstanceDynamic.SetVectorParameterValue` _returnvalue "Color" (`self.CubeColor`)))

(event `self.OnFixedTick`
  (params (Inputs :type "SquareInputs Structure"))
  (bind _result (`/Engine/EditorBlueprintResources/StandardMacros.DecrementInt` (`self.CounterTimer`))
    (:`  `
      (set `self.CounterTimer` (`KismetMathLibrary.Max` _result))
      (if (<= (`self.CounterTimer`) 0)
        (if (`.A` (break `SquareInputs` Inputs))
          (`/Engine/EditorBlueprintResources/StandardMacros.IncrementInt` (`self.Counter`)
            (:`  `
              (set `self.CounterTimer` (`self.CounterTimerMax`)))))))))

(event `self.OnViewTick`
  (if (> (`self.Counter`) 0)
    (`TextRenderComponent.K2_SetText` (`self.PlayerTag`) (`|FormatText` "Coins: {n}" (`self.Counter`)))
    (`SceneComponent.SetVisibility` (`self.PlayerTag`) true false)
    (else
      (`SceneComponent.SetVisibility` (`self.PlayerTag`) false false))))

(fn `UserConstructionScript`)