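; Game state for the Square mode that provides a shared top-down camera following the center of four square actors.
; On begin play, it spawns a camera actor, collects the squares by index and makes the camera player 0's view target, using next-tick delays between setup stages.
; Each tick, it moves the camera to the squares' average XY position at a fixed height, facing straight down.
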(event `self.ReceiveBeginPlay`
  (`parent.ReceiveBeginPlay`)
  (`KismetSystemLibrary.DelayUntilNextTick`)
  (bind _returnvalue (`|SpawnActorFromClass` "/Script/Engine.CameraActor" (`self.GetTransform`) "Undefined" "MultiplyWithRoot" null null))
  (set `self.CameraActor` _returnvalue)
  (for _index (range 4)
    (`KismetArrayLibrary.Array_Add` (`self.ActorsToOffset`) (`self.GetSquareActor` _index)))
  (`KismetSystemLibrary.DelayUntilNextTick`)
  (`PlayerController.SetViewTargetWithBlend` (`GameplayStatics.GetPlayerController` 0) (`self.CameraActor`) 0.0 "VTBlend_Linear" 0.0 false))

(event `self.ReceiveTick`
  (params (DeltaSeconds :type "Float (single-precision)"))
  (`parent.ReceiveTick` DeltaSeconds)
  (`/Engine/EditorBlueprintResources/StandardMacros.IsValid` (`self.CameraActor`)
    (:`Is Valid`
      (`self.UpdateCamera`))))

(fn `UpdateCamera`
  (bind _returnvalue (`GameplayStatics.GetActorArrayAverageLocation` (`self.ActorsToOffset`)))
  (`self.K2_SetActorLocation` (`self.CameraActor`) (`KismetMathLibrary.MakeVector` (.x _returnvalue) (.y _returnvalue) 900.0) false false)
  (`self.K2_SetActorRotation` (`self.CameraActor`) (struct :`Pitch` -90.0) false))

(fn `UserConstructionScript`)