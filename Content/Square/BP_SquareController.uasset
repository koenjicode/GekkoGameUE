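; BP_SquareController is the controller for the Square game mode, handling HUD setup and debug save/load input.
; On BeginPlay it creates WBP_SquareHUD for the first player controller, stores the reference and adds it to the viewport.
; Two debug keys cast GekkoGameState to SquareGameState and call SaveState and LoadState.
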(event EventBeginPlay
  (|CallParentFunction)
  (bind _returnvalue (UserInterface|CreateWidget "/Game/Square/WBP_SquareHUD.WBP_SquareHUD_C" (Game|GetPlayerController 0)))
  (bind _output_get (Variables|Default|SetSquareHUD _returnvalue))
  (Utilities|IsValid _output_get
    (:Is%20Valid
      (UserInterface|Viewport|AddtoViewport (Variables|Default|GetSquareHUD) 0))))

(event EventTick
  (params (DeltaSeconds :type Float%20%28single-precision%29)))

(event Input|KeyboardEvents|DebugKey8
  (params (Key :type Key%20Structure :default "None") (ActionValue :type Input%20Action%20Value%20Structure))
  (:Pressed
    (Class|SquareGameState|SaveState (.AsSquare%20Game%20State (Utilities|Casting|CastToSquareGameState (Variables|Default|GetGekkoGameState))))))

(event Input|KeyboardEvents|DebugKey9
  (params (Key :type Key%20Structure :default "None") (ActionValue :type Input%20Action%20Value%20Structure))
  (:Pressed
    (Class|SquareGameState|LoadState (.AsSquare%20Game%20State (Utilities|Casting|CastToSquareGameState (Variables|Default|GetGekkoGameState))))))

(fn ConstructionScript
  (|CallParentFunction))